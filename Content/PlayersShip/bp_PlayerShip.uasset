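; Player's ship that can be summoned, boarded, piloted and exited, and hides itself when the player strays too far.
; Overlap zones show prompts; interacting toggles ShipControls piloting, leveling the ship on release, or starts a screen fade for teleporting.
; Downward traces set the exit point and keep the beam's entrance trigger on the ground.
; BeginPlay links the first-person character to ShipControls and attaches a spawned bounty director.
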(event `self.ReceiveBeginPlay`
  (bind _shipcontrols (`self.ShipControls`))
  (bind _asbp_first_person_character (cast `/Game/FirstPerson/Blueprints/BP_FirstPersonCharacter` (`GameplayStatics.GetPlayerCharacter` 0)))
  (bind _output_get (set `self.BP_FirstPersonCharacter` _asbp_first_person_character))
  (`TheNewWestProjectCharacter.SetShipControlComp` _output_get _shipcontrols)
  (`ShipControlComponent.SetPlayer` _shipcontrols _output_get)
  (`ShipControlComponent.SetSeatAnchor` _shipcontrols (`self.SeatLocation`))
  (bind _returnvalue (`|SpawnActorFromClass` "/Game/PlayersShip/BP_BountyDirector.BP_BountyDirector_C" (`SceneComponent.K2_GetComponentToWorld` (`self.BountyDisplaySpawn`)) "AlwaysSpawn" "MultiplyWithRoot" null null))
  (`self.K2_AttachToComponent` _returnvalue (`self.BountyDisplaySpawn`) "None" "SnapToTarget" "SnapToTarget" "SnapToTarget" true))

(event `self.Interact_ControlPanel.OnComponentBeginOverlap`
  (params (OverlappedComponent :type "PrimitiveComponent Object Reference") (OtherActor :type "Actor Object Reference") (OtherComp :type "PrimitiveComponent Object Reference") (OtherBodyIndex :type Integer) (bFromSweep :type Boolean) (SweepResult :type "HitResult Structure (by ref)"))
  ;[0 1 0.7891 0.38] Ship Controls
  (if (`self.ActorHasTag` OtherActor "Player")
    (`WidgetComponent.SetWidget` (`self.ControlInteractPromt`) (`/Game/FirstPerson/Blueprints/BP_FirstPersonCharacter.WBP_InteractionPrompt` (`self.BP_FirstPersonCharacter`)))
    (set `self.playerInRangeOfControls` true)))

(event `self.Interact_ControlPanel.OnComponentEndOverlap`
  (params (OverlappedComponent :type "PrimitiveComponent Object Reference") (OtherActor :type "Actor Object Reference") (OtherComp :type "PrimitiveComponent Object Reference") (OtherBodyIndex :type Integer))
  ;[0 1 0.7891 0.38] Ship Controls
  (if (`self.ActorHasTag` OtherActor "Player")
    (`WidgetComponent.SetWidget` (`self.ControlInteractPromt`) null)
    (set `self.playerInRangeOfControls` false)))

(event `self.Interact_Exit.OnComponentBeginOverlap`
  (params (OverlappedComponent :type "PrimitiveComponent Object Reference") (OtherActor :type "Actor Object Reference") (OtherComp :type "PrimitiveComponent Object Reference") (OtherBodyIndex :type Integer) (bFromSweep :type Boolean) (SweepResult :type "HitResult Structure (by ref)"))
  ;[1 0.3842 0.2339 0.615] Exit
  (if (`self.ActorHasTag` OtherActor "Player")
    (`WidgetComponent.SetWidget` (`self.ExitInteractPromt`) (`/Game/FirstPerson/Blueprints/BP_FirstPersonCharacter.WBP_InteractionPrompt` (`self.BP_FirstPersonCharacter`)))
    (set `self.playerInRangeOfExit` true)))

(event `self.Interact_Exit.OnComponentEndOverlap`
  (params (OverlappedComponent :type "PrimitiveComponent Object Reference") (OtherActor :type "Actor Object Reference") (OtherComp :type "PrimitiveComponent Object Reference") (OtherBodyIndex :type Integer))
  ;[1 0.3842 0.2339 0.615] Exit
  (if (`self.ActorHasTag` OtherActor "Player")
    (`WidgetComponent.SetWidget` (`self.ExitInteractPromt`) null)
    (set `self.playerInRangeOfExit` false)))

(event `self.ReceiveTick`
  (params (DeltaSeconds :type "Float (single-precision)"))
  (bind _exitinteractpromt (`self.ExitInteractPromt`))
  (`self.DismissShip`)
  (`self.UpdateEntranceLocation`)
  ;[1 1 1] Exit Prompt Rotation
  (if (`self.playerInRangeOfExit`)
    (`SceneComponent.K2_SetWorldRotation` _exitinteractpromt (`KismetMathLibrary.FindLookAtRotation` (`SceneComponent.K2_GetComponentLocation` _exitinteractpromt) (`SceneComponent.K2_GetComponentLocation` (`TheNewWestProjectCharacter.FirstPersonCameraComponent` (`self.BP_FirstPersonCharacter`)))) false false)))

(event `self.EnterInteraction.OnComponentBeginOverlap`
  (params (OverlappedComponent :type "PrimitiveComponent Object Reference") (OtherActor :type "Actor Object Reference") (OtherComp :type "PrimitiveComponent Object Reference") (OtherBodyIndex :type Integer) (bFromSweep :type Boolean) (SweepResult :type "HitResult Structure (by ref)"))
  ;[0.9374 1 0.2172 0.521] Entrance
  (if (`self.ActorHasTag` OtherActor "Player")
    (`WidgetComponent.SetWidget` (`self.EnterInteractPrompt`) (`/Game/FirstPerson/Blueprints/BP_FirstPersonCharacter.WBP_InteractionPrompt` (`self.BP_FirstPersonCharacter`)))
    (set `self.playerInRangeOfEntrance` true)))

(event `self.EnterInteraction.OnComponentEndOverlap`
  (params (OverlappedComponent :type "PrimitiveComponent Object Reference") (OtherActor :type "Actor Object Reference") (OtherComp :type "PrimitiveComponent Object Reference") (OtherBodyIndex :type Integer))
  ;[0.9374 1 0.2172 0.521] Entrance
  (if (`self.ActorHasTag` OtherActor "Player")
    (`WidgetComponent.SetWidget` (`self.EnterInteractPrompt`) null)
    (set `self.playerInRangeOfEntrance` false)))

(fn `CallShip`
  (bind _bp_firstpersoncharacter (`self.BP_FirstPersonCharacter`))
  (if (not (`SceneComponent.bVisible` (`self.ShipCollision`)))
    (`self.K2_SetActorLocation` (`KismetMathLibrary.MakeVector` (.x (+ (`self.K2_GetActorLocation` _bp_firstpersoncharacter) (* (`self.GetActorForwardVector` _bp_firstpersoncharacter) (480.0 480.0 0.0)))) (.y (+ (`self.K2_GetActorLocation` _bp_firstpersoncharacter) (* (`self.GetActorForwardVector` _bp_firstpersoncharacter) (480.0 480.0 0.0)))) 8000.0) false true)
    (`SceneComponent.K2_SetWorldRotation` (`self.CapsuleComponent`) (`self.K2_GetActorRotation` (`self.BP_FirstPersonCharacter`)) false false)
    (`SceneComponent.SetVisibility` (`self.ShipCollision`) true true)))

(fn `DismissShip`
  (if (and (> (`KismetMathLibrary.Vector_Distance` (`self.K2_GetActorLocation` (`self.BP_FirstPersonCharacter`)) (`self.K2_GetActorLocation`)) 6000.0) (`SceneComponent.bVisible` (`self.ShipCollision`)))
    (`SceneComponent.SetVisibility` (`self.ShipCollision`) false true)
    (`self.K2_SetActorLocation` (0.0 0.0 0.0) false true)))

(fn `InteractionTriggered`
  (bind _returnvalue (`SceneComponent.K2_GetComponentLocation` (`self.ExitLineTrace`)))
  (if (`self.playerInRangeOfControls`)
    (bind _returnvalue_2 (`TheNewWestProjectCharacter.GetIsPlayerControllingShip` (`self.BP_FirstPersonCharacter`)))
    (bind _returnvalue_3 (not _returnvalue_2))
    (if (not _returnvalue_3)
      ;[1 0 0.126 0.385] Stop Controlling Ship
      (`self.K2_SetActorRotation` (`KismetMathLibrary.MakeRotator` 0.0 0.0 (.yaw (`self.K2_GetActorRotation`)))))
    (`ShipControlComponent.SetPlayerControllingShip` (`self.ShipControls`) _returnvalue_3)
    (`TheNewWestProjectCharacter.ToggleShipControlling` (`self.BP_FirstPersonCharacter`))
    (elif (`self.playerInRangeOfExit`)
      (`/Game/FirstPerson/Blueprints/BP_FirstPersonCharacter.PlayFadeScreen` (`self.BP_FirstPersonCharacter`) self)
      (bind (_outhit _returnvalue_4) (`KismetSystemLibrary.LineTraceSingle` _returnvalue (- _returnvalue (0.0 0.0 10000.0)) "TraceTypeQuery1" true))
      (set `self.canExit` _returnvalue_4)
      (set `self.ExitLocation` (`.Location` (`GameplayStatics.BreakHitResult` _outhit)))
      (elif (`self.playerInRangeOfEntrance`)
        (`/Game/FirstPerson/Blueprints/BP_FirstPersonCharacter.PlayFadeScreen` (`self.BP_FirstPersonCharacter`) self)))))

(fn `TeleportPlayer`
  (bind _bp_firstpersoncharacter (`self.BP_FirstPersonCharacter`))
  (if (and (`self.playerInRangeOfExit`) (`self.canExit`))
    (`self.K2_SetActorLocation` (`self.BP_FirstPersonCharacter`) (+ (`self.ExitLocation`) (0.0 0.0 75.0)) false true)
    (set `self.canExit` false)
    (elif (`self.playerInRangeOfEntrance`)
      (`self.K2_SetActorLocation` _bp_firstpersoncharacter (`SceneComponent.K2_GetComponentLocation` (`self.EnteranceLoc`)) false true)
      (`Controller.SetControlRotation` (`self.GetController` _bp_firstpersoncharacter) (`self.K2_GetActorRotation` self)))))

(fn `UpdateEntranceLocation`
  (bind _returnvalue (`SceneComponent.K2_GetComponentLocation` (`self.NS_ShipBeam`)))
  (bind _outhit (`KismetSystemLibrary.LineTraceSingle` :`Start` _returnvalue :`End` (- _returnvalue (0.0 0.0 10000.0)) :`TraceChannel` "TraceTypeQuery1" :`DrawTime` 1.0))
  (bind (_bblockinghit _binitialoverlap _time _distance _location) (`GameplayStatics.BreakHitResult` _outhit))
  (`SceneComponent.K2_SetWorldLocation` (`self.EnterInteraction`) _location false true)
  (`SceneComponent.K2_SetWorldRotation` (`self.EnterInteraction`) (`KismetMathLibrary.FindLookAtRotation` _location (`self.K2_GetActorLocation` (`self.BP_FirstPersonCharacter`))) false false))

(fn `UserConstructionScript`)