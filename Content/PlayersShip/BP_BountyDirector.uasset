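; Bounty director actor on the player's ship that shows bounty information and triggers bounty progression updates.
; An overlap of the InteractionBox by an actor tagged Player calls UpdateBountyProgression, whose logic is not defined in these graphs.
; The UpdateBountyDisplay event writes the title and description from GetBountyTitle and GetBountyDescription into the WBP_BountyDisplay widget on its BountyDisplay component.
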(event `self.UpdateBountyDisplay`
  (bind _aswbp_bounty_display (cast `/Game/PlayersShip/Widgets/WBP_BountyDisplay` (`WidgetComponent.GetWidget` (`self.BountyDisplay`))))
  (`|ExecutionSequence`
    (:`then_0`
      (bind _returnvalue (`self.GetBountyTitle`))
      (set `TextBlock.Text` (`KismetTextLibrary.Conv_StringToText` _returnvalue) (`/Game/PlayersShip/Widgets/WBP_BountyDisplay.MBTitle` _aswbp_bounty_display)))
    (:`then_1`
      (bind _returnvalue_2 (`self.GetBountyDescription`))
      (set `TextBlock.Text` (`KismetTextLibrary.Conv_StringToText` _returnvalue_2) (`/Game/PlayersShip/Widgets/WBP_BountyDisplay.MBDesc` _aswbp_bounty_display)))))

(event `self.InteractionBox.OnComponentBeginOverlap`
  (params (OverlappedComponent :type "PrimitiveComponent Object Reference") (OtherActor :type "Actor Object Reference") (OtherComp :type "PrimitiveComponent Object Reference") (OtherBodyIndex :type Integer) (bFromSweep :type Boolean) (SweepResult :type "HitResult Structure (by ref)"))
  (if (`self.ActorHasTag` OtherActor "Player")
    (`self.UpdateBountyProgression`)))

(fn `UserConstructionScript`)