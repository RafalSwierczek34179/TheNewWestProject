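; BP_Enemy is an AI-controlled enemy that detects the player through a VisionRadius overlap component.
; On BeginPlay it registers itself as RelatedEnemy on its BP_AIController.
; Player-tagged actors entering the radius are passed to the controller as its Player, which is cleared when they leave.
; LookAtPlayer turns the enemy toward a given location on yaw only by keeping its own Z height.
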(event `self.ReceiveBeginPlay`
  (bind _asbp_aicontroller (cast `/Game/AI/BP_AIController` (`AIBlueprintHelperLibrary.GetAIController` self)))
  (set `/Game/AI/BP_AIController.RelatedEnemy` self _asbp_aicontroller))

(event `self.VisionRadius.OnComponentBeginOverlap`
  (params (OverlappedComponent :type "PrimitiveComponent Object Reference") (OtherActor :type "Actor Object Reference") (OtherComp :type "PrimitiveComponent Object Reference") (OtherBodyIndex :type Integer) (bFromSweep :type Boolean) (SweepResult :type "HitResult Structure (by ref)"))
  (if (`self.ActorHasTag` OtherActor "Player")
    (bind _asbp_aicontroller (cast `/Game/AI/BP_AIController` (`AIBlueprintHelperLibrary.GetAIController` self)))
    (bind _asbp_first_person_character (cast `/Game/FirstPerson/Blueprints/BP_FirstPersonCharacter` OtherActor))
    (set `/Game/AI/BP_AIController.player` _asbp_first_person_character _asbp_aicontroller)))

(event `self.VisionRadius.OnComponentEndOverlap`
  (params (OverlappedComponent :type "PrimitiveComponent Object Reference") (OtherActor :type "Actor Object Reference") (OtherComp :type "PrimitiveComponent Object Reference") (OtherBodyIndex :type Integer))
  (if (`self.ActorHasTag` OtherActor "Player")
    (bind _asbp_aicontroller (cast `/Game/AI/BP_AIController` (`AIBlueprintHelperLibrary.GetAIController` self)))
    (set `/Game/AI/BP_AIController.player` null _asbp_aicontroller)))

(fn `LookAtPlayer`
  (params (playerLocation :type "Vector Structure"))
  (bind (_x _y) (`KismetMathLibrary.BreakVector3f` playerLocation))
  (bind _returnvalue (`self.K2_GetActorLocation` self))
  (`self.K2_SetActorRotation` self (`KismetMathLibrary.FindLookAtRotation` _returnvalue (`KismetMathLibrary.MakeVector` _x _y (`.Z` (`KismetMathLibrary.BreakVector3f` _returnvalue)))) false))

(fn `UserConstructionScript`)